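; Interactable chest that opens once and shows a text prompt while the player character is nearby.
; The Interact event runs through a DoOnce to play separate non-looping animations on the bottom and top skeletal meshes.
; Box overlap with BP_ThirdPersonCharacter shows or hides the TextRender, independently of whether the chest has already been used.
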(event OnComponentBeginOverlap(Box)
  (params (OverlappedComponent :type Primitive%20Component%20Object%20Reference) (OtherActor :type Actor%20Object%20Reference) (OtherComp :type Primitive%20Component%20Object%20Reference) (OtherBodyIndex :type Integer) (bFromSweep :type Boolean) (SweepResult :type Hit%20Result%20Structure%20%28by%20ref%29))
  (Utilities|Casting|CastToBP_ThirdPersonCharacter OtherActor)
  (Development|SetHiddeninGame (Variables|Default|GetTextRender) false false))

(event OnComponentEndOverlap(Box)
  (params (OverlappedComponent :type Primitive%20Component%20Object%20Reference) (OtherActor :type Actor%20Object%20Reference) (OtherComp :type Primitive%20Component%20Object%20Reference) (OtherBodyIndex :type Integer))
  (Utilities|Casting|CastToBP_ThirdPersonCharacter OtherActor)
  (Development|SetHiddeninGame (Variables|Default|GetTextRender) true false))

(event EventInteract
  (Utilities|FlowControl|DoOnce false
    (:Completed
      (Components|Animation|PlayAnimation (Variables|Default|GetSkeletalMesh) "/Game/Chest/source/chest_anim_bot_Anim.chest_anim_bot_Anim" false)
      (Components|Animation|PlayAnimation (Variables|Default|GetSkeletalMesh1) "/Game/Chest/source/chest_anim_top_Anim.chest_anim_top_Anim" false))))

(fn ConstructionScript)