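; Interactable chest actor that plays its opening animations when its Interact event fires.
; Bottom and top are separate skeletal meshes, each playing a non-looping animation.
; A DoOnce gates the event but resets immediately after starting playback, so repeated interactions replay the animations.
; Box overlap shows a widget while BP_ThirdPersonCharacter is inside and hides it on exit.
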(event OnComponentBeginOverlap(Box)
  (params (OverlappedComponent :type Primitive%20Component%20Object%20Reference) (OtherActor :type Actor%20Object%20Reference) (OtherComp :type Primitive%20Component%20Object%20Reference) (OtherBodyIndex :type Integer) (bFromSweep :type Boolean) (SweepResult :type Hit%20Result%20Structure%20%28by%20ref%29))
  (Utilities|Casting|CastToBP_ThirdPersonCharacter OtherActor)
  (Rendering|SetVisibility (Variables|Default|GetWidget) true false))

(event OnComponentEndOverlap(Box)
  (params (OverlappedComponent :type Primitive%20Component%20Object%20Reference) (OtherActor :type Actor%20Object%20Reference) (OtherComp :type Primitive%20Component%20Object%20Reference) (OtherBodyIndex :type Integer))
  (Utilities|Casting|CastToBP_ThirdPersonCharacter OtherActor)
  (Rendering|SetVisibility (Variables|Default|GetWidget) false false))

(event EventInteract
  (Utilities|FlowControl|DoOnce false :!label _label
    (:Completed
      (Components|Animation|PlayAnimation (Variables|Default|GetSkeletalMesh) "/Game/Chest/chest_anim_bot_Anim.chest_anim_bot_Anim" false)
      (Components|Animation|PlayAnimation (Variables|Default|GetSkeletalMesh1) "/Game/Chest/chest_anim_top_Anim.chest_anim_top_Anim" false)
      (goto _label Reset))))

(fn ConstructionScript)