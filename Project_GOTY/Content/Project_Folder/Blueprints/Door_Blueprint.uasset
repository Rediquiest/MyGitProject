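; Interactive hinged door that opens and closes with sound when the player presses Interaction nearby.
; A Box trigger enables input and shows a prompt widget while overlapped.
; Each press flips the Closed flag to play or reverse a Timeline that drives the door's yaw.
; Timeline updates recompute Closed from the angle, and two DoOnce gates, reset by the Timeline, limit repeat triggers.
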(event OnComponentBeginOverlap(Box)
  (params (OverlappedComponent :type Primitive%20Component%20Object%20Reference) (OtherActor :type Actor%20Object%20Reference) (OtherComp :type Primitive%20Component%20Object%20Reference) (OtherBodyIndex :type Integer) (bFromSweep :type Boolean) (SweepResult :type Hit%20Result%20Structure%20%28by%20ref%29))
  (Input|EnableInput (Game|GetPlayerController 0))
  (Rendering|SetVisibility (Variables|Default|GetWidget) true false))

(event OnComponentEndOverlap(Box)
  (params (OverlappedComponent :type Primitive%20Component%20Object%20Reference) (OtherActor :type Actor%20Object%20Reference) (OtherComp :type Primitive%20Component%20Object%20Reference) (OtherBodyIndex :type Integer))
  (Input|DisableInput (Game|GetPlayerController 0))
  (Rendering|SetVisibility (Variables|Default|GetWidget) false false))

(event Input|ActionEvents|InputActionInteraction
  (params (Key :type Key%20Structure :default "None"))
  (:Pressed
    (bind _output_get (Variables|Default|SetClosed (not (Variables|Default|GetClosed))))
    (if _output_get
      (Utilities|FlowControl|DoOnce false :!label _label
        (:Completed
          (Audio|SpawnSound2D "/Game/Project_Folder/Sounds/Door_Open.Door_Open" 1.0 1.0 0.0 0)
          (bind _dooropen (Timeline|Timeline Play)
            (:Update
              (Transformation|SetRelativeRotation (Variables|Default|GetDoor) (Math|Rotator|MakeRotator 0.0 0.0 _dooropen) false false)
              (Variables|Default|SetClosed (> _dooropen 89.0))
              (goto _label_2 Reset))
            (:Finished
              (goto _label Reset)))))
      (else
        (Utilities|FlowControl|DoOnce false :!label _label_2
          (:Completed
            (Audio|SpawnSound2D "/Game/Project_Folder/Sounds/Door_Close.Door_Close" 1.0 1.0 0.0 0)
            (Timeline|Timeline Reverse)))))))

(fn ConstructionScript)