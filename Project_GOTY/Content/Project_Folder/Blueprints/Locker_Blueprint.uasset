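; Locker hiding spot that Ethan can enter and leave with the Hiding input while inside its trigger box.
; Box overlaps enable input and gate the action, which toggles the character's visibility and collision, blends the view between locker and character, and plays the door timeline.
; While hiding, mouse and gamepad look feed clamped pitch and yaw, applied to the locker camera by a self-recalling Delay loop instead of Tick.
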(event OnComponentBeginOverlap(Box)
  (params (OverlappedComponent :type Primitive%20Component%20Object%20Reference) (OtherActor :type Actor%20Object%20Reference) (OtherComp :type Primitive%20Component%20Object%20Reference) (OtherBodyIndex :type Integer) (bFromSweep :type Boolean) (SweepResult :type Hit%20Result%20Structure%20%28by%20ref%29))
  (bind _asbp_third_person_character (Utilities|Casting|CastToEthan_Blueprint OtherActor))
  (bind _output_get (Variables|Default|SetCharacter%20Referece _asbp_third_person_character))
  (Input|EnableInput (Game|GetPlayerController 0))
  (Components|Movement|StopMovementImmediately (Variables|/Script/Engine.Character|GetCharacterMovement _output_get))
  (Utilities|FlowControl|Gate true) ; enters at Open
)

(event OnComponentEndOverlap(Box)
  (params (OverlappedComponent :type Primitive%20Component%20Object%20Reference) (OtherActor :type Actor%20Object%20Reference) (OtherComp :type Primitive%20Component%20Object%20Reference) (OtherBodyIndex :type Integer))
  (bind _returnvalue (Game|GetPlayerController 0))
  (Utilities|Casting|CastToEthan_Blueprint OtherActor)
  (Input|EnableInput _returnvalue)
  (Utilities|FlowControl|Gate true) ; enters at Close
)

(event Custom|CustomEvent
  (if (Variables|Default|GetIs%20Hiding?)
    (Transformation|SetRelativeRotation (Variables|Default|GetCamera) (Math|Rotator|MakeRotator 0.0 (* (stale Input|AxisEvents|InputAxisLookUp/DownGamepad _output_get) -1.0) (stale Input|AxisEvents|InputAxisTurnRight/LeftGamepad _output_get)) false false)
    (Utilities|FlowControl|Delay 0.001)
    (CallFunction|MoveCamera)))

(event Custom|Move%20Camera
  (if (Variables|Default|GetIs%20Hiding?)
    (Transformation|SetRelativeRotation (Variables|Default|GetCamera) (Math|Rotator|MakeRotator 0.0 (* (stale Input|AxisEvents|InputAxisLookUp/DownMouse _output_get) -1.0) (stale Input|AxisEvents|InputAxisTurnRight/LeftMouse _output_get)) false false)
    (Utilities|FlowControl|Delay 0.001)
    (CallFunction|MoveCamera)))

(event Input|ActionEvents|InputActionHiding
  (params (Key :type Key%20Structure))
  (:Pressed
    (Utilities|FlowControl|Gate true :!label _label
      (:Exit
        (Utilities|FlowControl|Sequence
          (:then_0
            (CallFunction|ToggleHide)
            (CallFunction|MoveCamera)
            (Utilities|FlowControl|Delay 0.2)
            (Input|EnableInput (Game|GetPlayerController 0))
            (Components|Movement|StopMovementImmediately (Variables|/Script/Engine.Character|GetCharacterMovement (stale OnComponentBeginOverlap(Box) _output_get)))
            (goto _label Open))
          (:then_1
            (|OpenDoor)))))))

(event Input|AxisEvents|InputAxisLookUp/DownMouse
  (params (AxisValue :type Float%20%28single-precision%29))
  (if (Variables|Default|GetIs%20Hiding?)
    (bind _output_get (Variables|Default|SetPitch (Math|Float|Clamp(Float) (+ (Variables|Default|GetPitch) AxisValue) -2e+01 2e+01)))
    (else
      (Pawn|Input|AddControllerPitchInput (Variables|Default|GetCharacter%20Referece) AxisValue))))

(event Input|AxisEvents|InputAxisTurnRight/LeftMouse
  (params (AxisValue :type Float%20%28single-precision%29))
  (if (Variables|Default|GetIs%20Hiding?)
    (bind _output_get (Variables|Default|SetYaw (Math|Float|Clamp(Float) (+ (Variables|Default|GetYaw) AxisValue) -3e+01 3e+01)))
    (else
      (Pawn|Input|AddControllerYawInput (Variables|Default|GetCharacter%20Referece) AxisValue))))

(event Input|AxisEvents|InputAxisLookUp/DownGamepad
  (params (AxisValue :type Float%20%28single-precision%29))
  (if (Variables|Default|GetIs%20Hiding?)
    (bind _output_get (Variables|Default|SetPitch (Math|Float|Clamp(Float) (+ (Variables|Default|GetPitch) AxisValue) -2e+01 2e+01)))
    (else
      (Pawn|Input|AddControllerPitchInput (Variables|Default|GetCharacter%20Referece) AxisValue))))

(event Input|AxisEvents|InputAxisTurnRight/LeftGamepad
  (params (AxisValue :type Float%20%28single-precision%29))
  (if (Variables|Default|GetIs%20Hiding?)
    (bind _output_get (Variables|Default|SetYaw (Math|Float|Clamp(Float) (+ (Variables|Default|GetYaw) AxisValue) -3e+01 3e+01)))
    (else
      (Pawn|Input|AddControllerYawInput (Variables|Default|GetCharacter%20Referece) AxisValue))))

(fn ConstructionScript)

(fn ToggleHide
  (bind _returnvalue (Game|GetPlayerController 0))
  (bind _character_referece (Variables|Default|GetCharacter%20Referece))
  (if (Variables|Default|GetIs%20Hiding?)
    (Variables|Default|SetIs%20Hiding? false)
    (Audio|PlaySound2D "/Game/Project_Folder/Sounds/Locker.Locker" 1.0 1.0 0.0 0 0)
    (Rendering|SetActorHiddenInGame _character_referece false)
    (Collision|SetActorEnableCollision _character_referece true)
    (Game|Player|SetViewTargetwithBlend _returnvalue _character_referece 1.0 "VTBlend_Linear" 0.0 false)
    (else
      (Variables|Default|SetIs%20Hiding? true)
      (Audio|PlaySound2D "/Game/Project_Folder/Sounds/Locker.Locker" 1.0 1.0 0.0 0 0)
      (Rendering|SetActorHiddenInGame _character_referece true)
      (Collision|SetActorEnableCollision _character_referece false)
      (Game|Player|SetViewTargetwithBlend _returnvalue self 0.6 "VTBlend_Linear" 0.0 false))))