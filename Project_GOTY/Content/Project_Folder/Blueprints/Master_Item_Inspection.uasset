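; Base inspectable item actor that shows a prompt widget when the third-person character overlaps its sphere and can be picked up for close inspection.
; On inspect, it disables collision, attaches to the camera manager, slides into view, shows a name/description UI, and takes input from the player.
; Mouse drag or movement axes rotate it.
; The Interaction key detaches it, returns it to its stored BeginPlay transform, and restores collision and player input.
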(event OnComponentBeginOverlap(Sphere)
  (params (OverlappedComponent :type Primitive%20Component%20Object%20Reference) (OtherActor :type Actor%20Object%20Reference) (OtherComp :type Primitive%20Component%20Object%20Reference) (OtherBodyIndex :type Integer) (bFromSweep :type Boolean) (SweepResult :type Hit%20Result%20Structure%20%28by%20ref%29))
  (Utilities|Casting|CastToBP_ThirdPersonCharacter OtherActor)
  (Rendering|SetVisibility (Variables|Default|GetWidget) true false))

(event OnComponentEndOverlap(Sphere)
  (params (OverlappedComponent :type Primitive%20Component%20Object%20Reference) (OtherActor :type Actor%20Object%20Reference) (OtherComp :type Primitive%20Component%20Object%20Reference) (OtherBodyIndex :type Integer))
  (Utilities|Casting|CastToBP_ThirdPersonCharacter OtherActor)
  (Rendering|SetVisibility (Variables|Default|GetWidget) false false))

(event EventBeginPlay
  (Variables|Default|SetTransform (Transformation|GetActorTransform)))

(event EventInspectInterection
  (params (Player :type BP%20Third%20Person%20Character%20Object%20Reference) (Is%20Letter :type Boolean) (The%20Item :type Actor%20Object%20Reference))
  (bind _returnvalue (Game|GetPlayerController 0))
  (Variables|Default|SetPlayer Player)
  (Collision|SetActorEnableCollision false)
  (Collision|SetCollisionProfileName (Variables|Default|GetSphere) "NoCollision" true :!class /Script/Engine.PrimitiveComponent)
  (Transformation|AttachComponentToComponent (Variables|/Script/Engine.PlayerCameraManager|GetTransformComponent (Game|GetPlayerCameraManager 0)) "None" "KeepWorld" "KeepWorld" "KeepWorld" true)
  (bind _returnvalue_2 (UserInterface|CreateWidget "/Game/Project_Folder/Blueprints/Widgets/Inspection_Ui.Inspection_Ui_C" 0 (Variables|Default|GetItem%20Name) (Variables|Default|GetItem%20Description)))
  (bind _output_get (Variables|Default|SetInspect%20UI _returnvalue_2))
  (UserInterface|Viewport|AddtoViewport _output_get 0)
  (Components|MoveComponentTo (Variables|Default|GetDefaultSceneRoot) "100.000000,-5.000000,0.000000" "90.000000,0.000000,0.000000" false false 0.2 false)
  (Input|DisableInput (Variables|Default|GetPlayer) _returnvalue)
  (Input|EnableInput _returnvalue))

(event Input|ActionEvents|InputActionInteraction
  (params (Key :type Key%20Structure :default "None"))
  (bind _returnvalue (Game|GetPlayerController 0))
  (bind _transform (Variables|Default|GetTransform))
  (:Pressed
    (Transformation|DetachFromActor "KeepWorld" "KeepWorld" "KeepWorld")
    (Widget|RemovefromParent (Variables|Default|GetInspect%20UI))
    (Variables|Default|SetInspect%20UI 0)
    (Components|MoveComponentTo (Variables|Default|GetDefaultSceneRoot) (.location _transform) (.rotation _transform) false false 0.2 false)
    (Collision|SetActorEnableCollision true)
    (Collision|SetCollisionProfileName (Variables|Default|GetSphere) "OverlapAllDynamic" true :!class /Script/Engine.PrimitiveComponent)
    (Input|DisableInput _returnvalue)
    (Input|EnableInput (Variables|Default|GetPlayer) _returnvalue)))

(event Input|AxisEvents|InputAxisMoveForward/Backward
  (params (AxisValue :type Float%20%28single-precision%29))
  (if (!= AxisValue 0.0)
    (Transformation|SetActorRotation (Math|Rotator|CombineRotators (Transformation|GetActorRotation) (Math|Rotator|MakeRotator 0.0 (* AxisValue 1.0) 0.0)))))

(event Input|AxisEvents|InputAxisMoveRight/Left
  (params (AxisValue :type Float%20%28single-precision%29))
  (if (!= AxisValue 0.0)
    (Transformation|SetActorRotation (Math|Rotator|CombineRotators (Transformation|GetActorRotation) (Math|Rotator|MakeRotator 0.0 0.0 (* AxisValue 1.0))))))

(event Input|MouseEvents|MouseX
  (params (AxisValue :type Float%20%28single-precision%29))
  (if (Variables|Default|GetCan%20Rotate)
    (Transformation|SetActorRotation (Math|Rotator|CombineRotators (Transformation|GetActorRotation) (Math|Rotator|MakeRotator 0.0 0.0 (* AxisValue 2.0))))))

(event Input|MouseEvents|MouseY
  (params (AxisValue :type Float%20%28single-precision%29))
  (if (Variables|Default|GetCan%20Rotate)
    (Transformation|SetActorRotation (Math|Rotator|CombineRotators (Transformation|GetActorRotation) (Math|Rotator|MakeRotator 0.0 (* AxisValue -2.0) 0.0)))))

(event Input|MouseEvents|LeftMouseButton
  (params (Key :type Key%20Structure :default "None"))
  (:Pressed
    (Variables|Default|SetCan%20Rotate true))
  (:Released
    (Variables|Default|SetCan%20Rotate false)))

(fn ConstructionScript)