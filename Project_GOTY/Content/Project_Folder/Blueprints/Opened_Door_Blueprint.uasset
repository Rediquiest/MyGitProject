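; Interactive door that the Ethan character opens and closes with the Interaction input while standing inside its trigger box.
; Box overlap enables input, shows a prompt widget and opens a gate, and leaving reverses all three.
; Each press flip-flops a timeline that plays or reverses, lerping the mesh yaw between closed and open angles, with door sounds and an Ethan montage on opening.
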(event OnComponentBeginOverlap(Box)
  (params (OverlappedComponent :type Primitive%20Component%20Object%20Reference) (OtherActor :type Actor%20Object%20Reference) (OtherComp :type Primitive%20Component%20Object%20Reference) (OtherBodyIndex :type Integer) (bFromSweep :type Boolean) (SweepResult :type Hit%20Result%20Structure%20%28by%20ref%29))
  (bind _asbp_third_person_character (Utilities|Casting|CastToEthan_Blueprint OtherActor))
  (Input|EnableInput (Game|GetPlayerController 0))
  (Rendering|SetVisibility (Variables|Default|GetWidget) true false)
  (Utilities|FlowControl|Gate true) ; enters at Open
)

(event OnComponentEndOverlap(Box)
  (params (OverlappedComponent :type Primitive%20Component%20Object%20Reference) (OtherActor :type Actor%20Object%20Reference) (OtherComp :type Primitive%20Component%20Object%20Reference) (OtherBodyIndex :type Integer))
  (Utilities|Casting|CastToEthan_Blueprint OtherActor)
  (Input|DisableInput (Game|GetPlayerController 0))
  (Rendering|SetVisibility (Variables|Default|GetWidget) false false)
  (Utilities|FlowControl|Gate true) ; enters at Close
)

(event Input|ActionEvents|InputActionInteraction
  (params (Key :type Key%20Structure))
  (:Pressed
    (Utilities|FlowControl|Gate true
      (:Exit
        (Utilities|FlowControl|FlipFlop
          (:A
            (Audio|SpawnSound2D "/Game/Project_Folder/Sounds/Door_Open.Door_Open" 1.0 1.0 0.0 0)
            (Animation|PlayAnimMontage (stale OnComponentBeginOverlap(Box) _asbp_third_person_character) "/Game/Project_Folder/Characters/Animations/Animation_Montages/Open_Montage.Open_Montage" 1.0 "None")
            (bind _door_track (Timeline|Open/Close%20Door Play)
              (:Update
                (Transformation|SetRelativeRotation (Variables|Default|GetStaticMesh) (Math|Rotator|MakeRotator 0.0 0.0 (Math|Float|Lerp (Variables|Default|GetClosed%20Angel) (Variables|Default|GetOpen%20Angel) _door_track)) false false))))
          (:B
            (Audio|SpawnSound2D "/Game/Project_Folder/Sounds/Door_Close.Door_Close" 1.0 1.0 0.0 0)
            (Timeline|Open/Close%20Door Reverse)))))))

(fn ConstructionScript)