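; Key pickup actor that lets the third-person character collect a key with the Interaction input.
; Its Box overlap enables input, shows a prompt widget and opens a Gate; leaving reverses all three.
; Pressing Interaction through the open gate sets HasKey on the character, plays the pick-up montage, then after a short delay plays a sound and destroys the key.
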(event OnComponentBeginOverlap(Box)
  (params (OverlappedComponent :type Primitive%20Component%20Object%20Reference) (OtherActor :type Actor%20Object%20Reference) (OtherComp :type Primitive%20Component%20Object%20Reference) (OtherBodyIndex :type Integer) (bFromSweep :type Boolean) (SweepResult :type Hit%20Result%20Structure%20%28by%20ref%29))
  (bind _asbp_third_person_character (Utilities|Casting|CastToBP_ThirdPersonCharacter OtherActor))
  (Input|EnableInput (Game|GetPlayerController 0))
  (Rendering|SetVisibility (Variables|Default|GetWidget) true false)
  (Utilities|FlowControl|Gate true) ; enters at Open
)

(event OnComponentEndOverlap(Box)
  (params (OverlappedComponent :type Primitive%20Component%20Object%20Reference) (OtherActor :type Actor%20Object%20Reference) (OtherComp :type Primitive%20Component%20Object%20Reference) (OtherBodyIndex :type Integer))
  (Utilities|Casting|CastToBP_ThirdPersonCharacter OtherActor)
  (Input|DisableInput (Game|GetPlayerController 0))
  (Rendering|SetVisibility (Variables|Default|GetWidget) false false)
  (Utilities|FlowControl|Gate true) ; enters at Close
)

(event Input|ActionEvents|InputActionInteraction
  (params (Key :type Key%20Structure :default "None"))
  (:Pressed
    (Utilities|FlowControl|Gate true
      (:Exit
        (Variables|/Game/BP_ThirdPersonCharacter.BP_ThirdPersonCharacter_C|SetHasKey? (stale OnComponentBeginOverlap(Box) _asbp_third_person_character) true)
        (Animation|PlayAnimMontage (stale OnComponentBeginOverlap(Box) _asbp_third_person_character) "/Game/Project_Folder/Characters/Animations/Animation_Montages/Pick_Up_Montage.Pick_Up_Montage" 1.0 "None")
        (Utilities|FlowControl|Delay 0.3)
        (Audio|PlaySoundatLocation "/Game/Project_Folder/Sounds/Key_Pick_Up.Key_Pick_Up" (Transformation|GetActorLocation) "0, 0, 0" 1.0 1.0 0.0 0 0 0 0)
        (Actor|DestroyActor)))))

(fn ConstructionScript)